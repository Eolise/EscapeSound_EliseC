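; BP_Door is a wooden door actor that swings open and closed when its Interact event fires.
; BeginPlay stores the starting rotation, and each Interact alternates through a FlipFlop between playing and reversing the Opening timeline with the matching wood sound.
; The timeline update lerps the whole actor's rotation to 90 degrees of negative yaw from the stored start, so the swing is relative to its placed orientation.
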(event `self.ReceiveBeginPlay`
  (set `self.StartingRotation` (`self.K2_GetActorRotation`)))

(event `/Game/Blueprints/BPI_Interaction.Interact`
  (bind (_startingrotation_roll _startingrotation_pitch _startingrotation_yaw) (`KismetMathLibrary.BreakRotator` (`self.StartingRotation`)))
  (`/Engine/EditorBlueprintResources/StandardMacros.FlipFlop`
    (:`A`
      (`GameplayStatics.PlaySoundAtLocation` "/Game/Sounds/FX/Door_Wood_Open.Door_Wood_Open" (`SceneComponent.K2_GetComponentLocation` (`self.StaticMeshComponent0`)) (struct) 1.0 1.0 0.0 null null null null)
      (bind (_direction _newtrack_0) (`Timeline|Opening` :!label _label)
        (:`Update`
          (`self.K2_SetActorRotation` (`KismetMathLibrary.RLerp` (`self.StartingRotation`) (`KismetMathLibrary.MakeRotator` _startingrotation_roll _startingrotation_pitch (+ _startingrotation_yaw -90.0)) _newtrack_0 true)))))
    (:`B`
      (`GameplayStatics.PlaySoundAtLocation` "/Game/Sounds/FX/Door_Wood_Close.Door_Wood_Close" (`SceneComponent.K2_GetComponentLocation` (`self.StaticMeshComponent0`)) (struct) 1.0 1.0 0.0 null null null null)
      (goto _label :!via `Reverse`))))

(fn `UserConstructionScript`)