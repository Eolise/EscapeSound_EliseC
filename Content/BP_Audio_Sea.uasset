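; Sea ambience actor that places its audio at the point on a spline nearest the player character.
; BeginPlay caches the third-person character, then moves the Audio and Arrow components to the closest spline location, raised slightly in Z.
; It calls MoveAudio before and shortly after that move, but the event is empty here, so the position updates only once.
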(event `self.ReceiveBeginPlay`
  (bind (_returnvalue_x _returnvalue_y _returnvalue_z) (`KismetMathLibrary.BreakVector` (`SplineComponent.FindLocationClosestToWorldLocation` (`self.Spline`) (`self.K2_GetActorLocation` (`self.As BP Third Person Character`)) "World")))
  (bind _asbp_third_person_character (cast `/Game/Blueprints/BP_ThirdPersonCharacter` (`GameplayStatics.GetPlayerCharacter` 0)))
  (set `self.As BP Third Person Character` _asbp_third_person_character)
  (`self.Move Audio`)
  (`SceneComponent.K2_SetWorldLocation` (`self.Audio`) (`KismetMathLibrary.MakeVector` _returnvalue_x _returnvalue_y (+ _returnvalue_z 50.0)) false false)
  (`SceneComponent.K2_SetWorldLocation` (`self.Arrow`) (`KismetMathLibrary.MakeVector` _returnvalue_x _returnvalue_y (+ _returnvalue_z 50.0)) false false)
  (`KismetSystemLibrary.Delay` 0.05)
  (`self.Move Audio`))

(event `Move Audio`)

(fn `UserConstructionScript`)